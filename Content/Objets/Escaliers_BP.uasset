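; Escaliers_BP is a staircase actor that moves between its placed position and an offset when its linked pressure plate (Plaque) is active.
; The construction script records the placed location as the default.
; Each tick it teleports one fiftieth of the Mouvement vector toward the offset while Plaque is active, or back otherwise, stopping within a small tolerance.
; Speed therefore depends on frame rate rather than delta time.
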(event `self.ReceiveTick`
  (params (DeltaSeconds :type "Float (single-precision)"))
  (bind _returnvalue (`self.K2_GetActorLocation`))
  (bind _default_location (`self.default location`))
  (bind _mouvement (`self.mouvement`))
  (bind _returnvalue_2 (/ _mouvement 50.0))
  (if (`/Game/Objets/PlaqueV2.activé ?` (`self.plaque`))
    (if (not (== _returnvalue (+ _default_location _mouvement)))
      (`self.K2_SetActorLocation` (+ _returnvalue _returnvalue_2) false true))
    (elif (not (== _default_location _returnvalue))
      (`self.K2_SetActorLocation` (- _returnvalue _returnvalue_2) false true))))

(event `self.ReceiveBeginPlay`)

(fn `UserConstructionScript`
  (set `self.default location` (`self.K2_GetActorLocation`)))