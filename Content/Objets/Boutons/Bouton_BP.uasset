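; Clickable button actor that signals a linked door (Porte) when left-clicked while TriggerBouton reports InTrigger.
; Its PressLeft prompt is forced visible and turned toward the player every Tick, then turns green on a valid click.
; The click plays a timeline that fades the dynamic material's Colour, sets the door's Cliqué flag and sinks the actor slightly on each update.
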(event `self.ReceiveBeginPlay`
  ;[1 1 1] Changer couleur bouton
  (bind _returnvalue (`PrimitiveComponent.CreateDynamicMaterialInstance` (`self.StaticMeshComponent`) 0 "/Game/Objets/Materials/Rouge.Rouge" "None"))
  (`self.EnableInput` (`GameplayStatics.GetPlayerController` 0)))

(event `self.ReceiveTick`
  (params (DeltaSeconds :type "Float (single-precision)"))
  (bind _press_left (`self.Press Left`))
  ;[1 1 1] Afficher texte
  (`SceneComponent.SetVisibility` (`self.Press Left`) true false)
  ;[1 1 1] Rotate texte face au joueur
  (`SceneComponent.K2_SetWorldRotation` _press_left (`KismetMathLibrary.FindLookAtRotation` (`SceneComponent.K2_GetComponentLocation` _press_left) (`self.K2_GetActorLocation` (`GameplayStatics.GetPlayerCharacter` 0))) false false))

(event `Key|LeftMouseButton`
  (params (Key :type "Key Structure"))
  ;[1 1 1] Changer couleur bouton
  (:`Pressed`
    (if (`/Game/Objets/TriggerBoxs/Trigger_Bouton.InTrigger?` (`self.Trigger_Bouton`))
      ;[1 1 1] Changer couleur texte
      (`TextRenderComponent.SetTextRenderColor` (`self.Press Left`) (`KismetMathLibrary.LinearColor_Quantize` (struct :`R` 0.063154 :`G` 0.760417 :`A` 1.0)))
      (bind (_direction _colourfade) (`Timeline|Timeline_0`)
        (:`Update`
          (`MaterialInstanceDynamic.SetVectorParameterValue` (stale `self.ReceiveBeginPlay` _returnvalue) "Colour" _colourfade)
          (set `/Game/Objets/Porte_BluePrint.Cliqué?` true (`self.Porte`))
          ;[1 1 1] Enfoncer le bouton
          (`self.K2_SetActorLocation` (- (`self.K2_GetActorLocation`) (0.0 0.0 0.05)) true))))))

(fn `UserConstructionScript`)