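; TriggerPlaque_BP is a trigger Blueprint that changes the colour of a referenced plate (Plaque) when an actor overlaps it.
; The overlap sets the Dessus flag, applies a dynamic instance of the Rouge material to the plate and enables player input on itself.
; While Dessus is set, Tick plays a timeline that drives the material's Colour parameter.
; Nothing in the graph clears the flag.
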(event `self.ReceiveActorBeginOverlap`
  (params (OtherActor :type "Actor Object Reference"))
  ;[1 1 1] Changer couleur plaque
  (set `self.Dessus?` true)
  (bind _returnvalue (`PrimitiveComponent.CreateDynamicMaterialInstance` (`StaticMeshActor.StaticMeshComponent` (`self.Plaque`)) 0 "/Game/Objets/Materials/Rouge.Rouge" "None"))
  (`self.EnableInput` (`GameplayStatics.GetPlayerController` 0)))

(event `self.ReceiveTick`
  (params (DeltaSeconds :type "Float (single-precision)"))
  ;[1 1 1] Changer couleur plaque
  (if (`self.Dessus?`)
    (bind (_direction _colourfade) (`Timeline|Timeline_0`)
      (:`Update`
        (`MaterialInstanceDynamic.SetVectorParameterValue` (stale `self.ReceiveActorBeginOverlap` _returnvalue) "Colour" _colourfade)))))

(fn `UserConstructionScript`)